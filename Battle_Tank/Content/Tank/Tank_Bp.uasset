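; Tank Blueprint that handles orbit camera input and firing.
; On BeginPlay it passes its Barrell and Turret components to setter functions defined outside these graphs.
; AxisAzimuth yaws AzimuthGimbel in world space, while AxisHorizontal pitches the SpringArm locally, keeping the two camera rotations on separate components.
; The Firing input calls a Firing function that is also defined outside these graphs.
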(event `self.ReceiveBeginPlay`
  (`self.SetBarrelReference` (`self.Barrell`))
  (`self.SetTurretReference` (`self.Turret`)))

(event `InputAxis|AxisAzimuth`
  (params (AxisValue :type "Float (single-precision)"))
  ;[1 1 1] Camera Input Binding
  (`SceneComponent.K2_AddWorldRotation` (`self.Azimuth_gimbel`) (`KismetMathLibrary.MakeRotator` 0.0 0.0 AxisValue) false false))

(event `InputAxis|AxisHorizontal`
  (params (AxisValue :type "Float (single-precision)"))
  ;[1 1 1] Camera Input Binding
  (`SceneComponent.K2_AddLocalRotation` (`self.SpringArm`) (`KismetMathLibrary.MakeRotator` 0.0 AxisValue) false false))

(event `InputAction|Firing`
  (params (Key :type "Key Structure"))
  ;[1 1 1] Camera Input Binding
  (:`Pressed`
    (`self.Firing`)))

(fn `UserConstructionScript`)